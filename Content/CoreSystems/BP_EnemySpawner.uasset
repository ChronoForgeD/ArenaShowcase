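; Enemy spawner that spawns a batch of BP_DrifterEnemy actors when the EncounterTrigger reports an encounter start.
; Spawn locations come from random level TargetPoints, with a retry check intended to avoid repeating the last-used index.
; Each enemy is tracked in ActiveEnemies and has its HealthComponent death delegate bound.
; A kill-counting event calls encounter completion at a hardcoded three kills, independent of the spawn count.
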(event Custom|CustomEvent
  (Development|PrintString "RemoveFromPool Fired")
  (bind _result (Math|Integer|IncrementInt (Variables|Default|GetKillCount))
    (:%20%20
      (if (== (Variables|Default|GetKillCount) 3)
        (Default|CallEncounterComplete)
        (Development|PrintString (Utilities|String|Append "Kill Count is now: " (Utilities|String|ToString(Integer) _result)))
        (Development|PrintString "Encounter Complete")
        (else
          (Development|PrintString (Utilities|String|Append "Kill Count is now: " (Utilities|String|ToString(Integer) _result))))))))

(event Custom|SpawnEnemies
  (Variables|Default|SetSpawnedCount 0)
  (Utilities|Array|Clear (Variables|Default|GetActiveEnemies))
  (for _index (range 0 (- (Variables|Default|GetEnemiesToSpawn) 1))
    (CallFunction|SpawnEnemy))
  (Development|PrintString "Spawned Enemies"))

(event EventBeginPlay
  (EventDispatchers|BindEventtoOnEncounterStarted (Variables|Default|GetEncounterTrigger) (delegate Custom|SpawnEnemies)))

(fn ConstructionScript)

(fn GetTargetPoints
  (bind _outactors (Actor|GetAllActorsOfClass "/Script/Engine.TargetPoint"))
  (bind _output_get (Variables|Default|SetTargetPoints _outactors :!label _label))
  (Development|PrintString (Utilities|String|Append "New Index " (Utilities|String|ToString(Integer) (.OutIndex (Utilities|Array|Random _output_get)))))
  (if (== (.OutIndex (Utilities|Array|Random _output_get)) (Variables|Default|GetLastUsedSpawn))
    (goto _label)
    (else
      (bind _output_get_2 (Variables|Default|SetLastUsedSpawn (.OutIndex (Utilities|Array|Random _output_get))))
      (Development|PrintString (Utilities|String|Append "Last Used Index: " (Utilities|String|ToString(Integer) _output_get_2)))
      (return (Transformation|GetActorLocation (.OutItem (Utilities|Array|Random _output_get)))))))

(fn SpawnEnemy
  (if (>= (Variables|Default|GetSpawnedCount) (Variables|Default|GetEnemiesToSpawn))
    (Development|PrintString "Max enemies spawned")
    (return 0)
    (else
      (bind _targetpointlocation (CallFunction|GetTargetPoints))
      (bind _returnvalue (Game|SpawnActorfromClass "/Game/Characters/Enemies/BP_DrifterEnemy.BP_DrifterEnemy_C" (Math|Transform|MakeTransform _targetpointlocation "0, 0, 0" "1.000000,1.000000,1.000000") "AlwaysSpawn" "MultiplyWithRoot" 0 0))
      (EventDispatchers|BindEventtoOnDeath (Actor|GetComponentbyClass _returnvalue "/Script/ArenaShowcase.HealthComponent") (EventDispatchers|CreateEvent :!event Custom|CustomEvent))
      (Development|PrintString "Bound To Death")
      (bind _returnvalue_2 (Utilities|Array|Add (Variables|Default|GetActiveEnemies) _returnvalue))
      (Variables|Default|SetSpawnedCount _returnvalue_2)
      (return _returnvalue))))
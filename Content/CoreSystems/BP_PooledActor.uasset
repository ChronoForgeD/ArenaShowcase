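; Base pooled actor that toggles between active and dormant states so it can be reused instead of spawned and destroyed.
; SetInUse shows or hides the actor, enables or disables its tick, and resets a time-to-live timer.
; When activated, the timer calls ReturnToPool after TimeToLive to deactivate it automatically; instances start inactive on BeginPlay.
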(event Custom|SetInUse
  (params (InUse :type Boolean))
  (bind _output_get (Variables|Default|SetInUse InUse))
  (Rendering|SetActorHiddenInGame (not _output_get))
  (Actor|Tick|SetActorTickEnabled InUse)
  (Utilities|Time|ClearandInvalidateTimerbyHandle (Variables|Default|GetTimeToLiveTimer))
  (if InUse
    (bind _returnvalue (Utilities|Time|SetTimerbyEvent (delegate Custom|ReturnToPool) (Variables|Default|GetTimeToLive)))
    (Variables|Default|SetTimeToLiveTimer _returnvalue)))

(event Custom|ReturnToPool
  (CallFunction|SetinUse false))

(event EventBeginPlay
  (CallFunction|SetinUse false))

(fn ConstructionScript)